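; Combat component for BP_ThirdPersonCharacterMain that runs networked katana attacks, parries and round-winning kills.
; Attacks play first- and third-person montages, then client camera traces send the hit actor and bone to the server.
; The server checks facing and status: perfect parry stuns the attacker, block negates damage.
; Other hits decrement the attacker component's own Health, driving victim screen effects, then dismemberment, ragdoll and a GameStateTest round win.
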(event Custom|Multicast_SuccessParry
  (params (SKMRef :type Skeletal%20Mesh%20Component%20Object%20Reference))
  (bind _character (Variables|REF|GetCharacter))
  (bind _clashlocation (Variables|/Game/Core/Character/BP_ThirdPersonCharacterMain.BP_ThirdPersonCharacterMain_C|GetClashLocation _character))
  ;[0.15 0.15 0.15 0.5] Parry Effect / Sound
  (Animation|Montage|PlayMontage SKMRef "/Game/Art/Characters/Mannequins/Anims/FPSAnim/AM_Parry_Hit.AM_Parry_Hit"
    (:OnNotifyBegin
      (Effects|SpawnEmitterAttached "/Game/Realistic_Starter_VFX_Pack_Vol2/Particles/Sparks/P_Sparks_E.P_Sparks_E" _clashlocation "None")
      (Audio|PlaySoundatLocation "/Game/SFX/Katana/Pary/SC_Parry_Katana.SC_Parry_Katana" (Variables|/Script/Engine.SceneComponent|GetRelativeLocation _clashlocation) "0, 0, 0" 1.0 1.0 0.0 0 0 0 0))))

(event Custom|Multicast_HItSound
  (params (Hit%20location :type Vector) (Rotation :type Rotator) (Hit%20Bones%20Name :type Name) (bloquer :type BP%20Third%20Person%20Character%20Main%20Object%20Reference))
  (bind _mesh (Variables|/Script/Engine.Character|GetMesh bloquer))
  ;[0.15 0.15 0.15 0.5] MultiCast Hit
  (if (< (Variables|STATS|GetHealth) 1.0)
    (CallFunction|Dissmebrement bloquer Hit%20Bones%20Name))
  (Audio|PlaySoundatLocation "/Game/SFX/Katana/Hit/SC_Hit_Katana.SC_Hit_Katana" Hit%20location "0, 0, 0" 1.0 1.0 0.0 0 0 0 0)
  (Niagara|SpawnSystemAttached "/Game/RealisticBlood/Hit/Niagara/NS_BulletHit_Sample.NS_BulletHit_Sample" _mesh Hit%20Bones%20Name Hit%20location Rotation "KeepWorldPosition" true)
  (Niagara|SpawnSystemAttached "/Game/RealisticBlood/Dripping/Niagara/NS_Dripping_Splash_Low.NS_Dripping_Splash_Low" _mesh Hit%20Bones%20Name Hit%20location Rotation "KeepWorldPosition" true))

(event Custom|Client_AttackTrace
  (bind _character (Variables|REF|GetCharacter))
  (bind _followcamera (Variables|/Game/Core/Character/BP_ThirdPersonCharacterMain.BP_ThirdPersonCharacterMain_C|GetFollowCamera _character))
  (bind _returnvalue (Transformation|GetWorldLocation _followcamera))
  (bind _returnvalue_2 (Math|Vector|GetForwardVector _followcamera))
  (bind _returnvalue_3 (* _returnvalue_2 4e+01))
  (bind _returnvalue_4 (+ _returnvalue _returnvalue_3))
  ;[0.15 0.15 0.15 0.5] Attack Trace / Box trace when attack
  (bind _outhit (Class|KismetSystemLibrary|BoxTraceSingleforObjects _returnvalue_4 (- _returnvalue_4 "0.000000,0.000000,100.000000") "40.000000,50.000000,50.000000" (Math|Rotator|MakeRotator 0.0 0.0 (.yaw (Math|Rotator|FindLookatRotation _returnvalue_4 (Transformation|GetWorldLocation _followcamera)))) (Utilities|Array|MakeArray "ObjectTypeQuery3") false 0 "ForOneFrame" true))
  (bind _asbp_third_person_character_main (Utilities|Casting|CastToBP_ThirdPersonCharacterMain (.HitActor (Collision|BreakHitResult _outhit))))
  (Variables|Default|SetAs%20BP%20Third%20Person%20Character%20Main _asbp_third_person_character_main)
  (if (!= _asbp_third_person_character_main self)
    (Development|PrintString (Utilities|String|ToString(Name) (.HitBoneName (Collision|BreakHitResult _outhit))))
    (CallFunction|ClientDetectBone)
    (CallFunction|ServerApplyDamage _asbp_third_person_character_main (.ImpactPoint (Collision|BreakHitResult _outhit)) (Variables|Default|GetTest2) (Math|Conversions|RotationFromXVector (.Normal (Collision|BreakHitResult _outhit))))))

(event Custom|Server_Stun
  ;[0.15 0.15 0.15 0.5] Stun
  (Variables|/Game/Core/Character/BP_ThirdPersonCharacterMain.BP_ThirdPersonCharacterMain_C|SetStatus (Variables|REF|GetCharacter) "NewEnumerator5")
  (Utilities|Time|SetTimerbyEvent (delegate Custom|RemoveStun) (Variables|Default|GetStunDuration)))

(event Custom|Multicast_LaunchAnimTPS
  (params (SKMMontage :type Skeletal%20Mesh%20Component%20Object%20Reference) (MontageToPlay :type Anim%20Montage%20Object%20Reference))
  (bind _character (Variables|REF|GetCharacter))
  (bind _swordtrail (Variables|/Game/Core/Character/BP_ThirdPersonCharacterMain.BP_ThirdPersonCharacterMain_C|GetSwordTrail _character))
  ;[0.15 0.15 0.15 0.5] Attack Anim System
  (Animation|Montage|PlayMontage SKMMontage MontageToPlay 1.5
    (:then
      (Utilities|FlowControl|Delay 0.1)
      (Components|Activation|Activate _swordtrail true)
      (Utilities|FlowControl|Delay (- (Variables|BlockSettings|GetAttackTraceDelay) 0.1))
      (Components|Activation|Deactivate _swordtrail))))

(event Custom|Client_LaunchAnimFPS
  (params (MontageToPlay :type Anim%20Montage%20Object%20Reference))
  (bind _character (Variables|REF|GetCharacter))
  (bind _swordtraillocal (Variables|/Game/Core/Character/BP_ThirdPersonCharacterMain.BP_ThirdPersonCharacterMain_C|GetSwordTrailLocal _character))
  ;[0.15 0.15 0.15 0.5] Attack Anim System
  (Animation|Montage|PlayMontage (Variables|/Game/Core/Character/BP_ThirdPersonCharacterMain.BP_ThirdPersonCharacterMain_C|GetMesh_Local (Variables|REF|GetCharacter)) MontageToPlay 1.5
    (:then
      (CallFunction|ClientAttackTrace)
      (Audio|PlaySound2D "/Game/SFX/Katana/Attaque/SC_Attaque_Katana.SC_Attaque_Katana" 1.0 1.0 0.0 0 0)
      (Utilities|FlowControl|Delay 0.1)
      (Components|Activation|Activate _swordtraillocal true)
      (Utilities|FlowControl|Delay (- (Variables|BlockSettings|GetAttackTraceDelay) 0.1))
      (Components|Activation|Deactivate _swordtraillocal))))

(event Custom|RemoveStun
  ;[0.15 0.15 0.15 0.5] Stun
  (Variables|/Game/Core/Character/BP_ThirdPersonCharacterMain.BP_ThirdPersonCharacterMain_C|SetStatus (Variables|REF|GetCharacter) "NewEnumerator4"))

(event Custom|Client_DetectBone
  (bind _character (Variables|REF|GetCharacter))
  (bind _followcamera (Variables|/Game/Core/Character/BP_ThirdPersonCharacterMain.BP_ThirdPersonCharacterMain_C|GetFollowCamera _character))
  (bind _returnvalue (Transformation|GetWorldLocation _followcamera))
  (bind _outhit (Collision|LineTraceForObjects _returnvalue (+ _returnvalue (* (Math|Vector|GetForwardVector _followcamera) 1.5e+02)) (Utilities|Array|MakeArray "ObjectTypeQuery4") false 0 "None"))
  (Variables|Default|SetTest2 (.HitBoneName (Collision|BreakHitResult _outhit))))

(event Custom|Server_LaunchAnimBlockTPS
  (params (SKMRef :type Skeletal%20Mesh%20Component%20Object%20Reference) (MontageToPlay :type Anim%20Montage%20Object%20Reference))
  ;[0.15 0.15 0.15 0.5] Block Anim System
  (CallFunction|MulticastLaunchAnimBlockTPS SKMRef MontageToPlay))

(event Custom|Client_LaunchAnimBlockFPS
  (params (MontageToPlay :type Anim%20Montage%20Object%20Reference))
  ;[0.15 0.15 0.15 0.5] Block Anim System
  (Animation|Montage|PlayMontage (Variables|/Game/Core/Character/BP_ThirdPersonCharacterMain.BP_ThirdPersonCharacterMain_C|GetMesh_Local (Variables|REF|GetCharacter)) MontageToPlay))

(event Custom|Multicast_LaunchAnimBlockTPS
  (params (SKMRef :type Skeletal%20Mesh%20Component%20Object%20Reference) (MontageToPlay :type Anim%20Montage%20Object%20Reference))
  ;[0.15 0.15 0.15 0.5] Block Anim System
  (Animation|Montage|PlayMontage SKMRef MontageToPlay))

(event Custom|Server_ParryStates
  (bind _character (Variables|REF|GetCharacter))
  ;[0.15 0.15 0.15 0.5] Block/Input
  (if (and (Utilities|Enum|Equal(Enum) (Variables|/Game/Core/Character/BP_ThirdPersonCharacterMain.BP_ThirdPersonCharacterMain_C|GetStatus _character) "NewEnumerator4") (not (Variables|Default|GetInParry)))
    (Utilities|FlowControl|Sequence
      (:then_0
        (Variables|Default|SetInParry true)
        (Variables|/Game/Core/Character/BP_ThirdPersonCharacterMain.BP_ThirdPersonCharacterMain_C|SetStatus _character "NewEnumerator6")
        (Utilities|FlowControl|Delay (Variables|BlockSettings|GetPerfectParryTimer))
        (Variables|/Game/Core/Character/BP_ThirdPersonCharacterMain.BP_ThirdPersonCharacterMain_C|SetStatus (Variables|REF|GetCharacter) "NewEnumerator3")
        (Utilities|FlowControl|Delay (- (Variables|BlockSettings|GetParryTimer) (Variables|BlockSettings|GetPerfectParryTimer)))
        (Variables|/Game/Core/Character/BP_ThirdPersonCharacterMain.BP_ThirdPersonCharacterMain_C|SetStatus (Variables|REF|GetCharacter) "NewEnumerator4")
        (Utilities|FlowControl|Delay (Utilities|Operators|Subtract (Variables|BlockSettings|GetBlockCooldown) (Variables|BlockSettings|GetParryTimer) (Variables|BlockSettings|GetPerfectParryTimer)))
        (Variables|Default|SetInParry false))
      (:then_1
        (CallFunction|ClientLaunchAnimBlockFPS "/Game/Art/Characters/Mannequins/Anims/FPSAnim/AM_Parry.AM_Parry")
        (CallFunction|ServerLaunchAnimBlockTPS (Variables|/Script/Engine.Character|GetMesh (Variables|REF|GetCharacter)) "/Game/Art/Characters/Mannequins/Anims/FPSAnim/AM_Parry.AM_Parry")))))

(event Custom|Multicast_Block
  (params (char :type BP%20Third%20Person%20Character%20Main%20Object%20Reference))
  (bind _mesh (Variables|/Script/Engine.Character|GetMesh char))
  (bind _returnvalue (Components|SkeletalMesh|GetAnimInstance _mesh))
  ;[0.15 0.15 0.15 0.5] Block and Parry
  (Animation|Montage|MontageStop _returnvalue 0.25 (Animation|Montage|GetCurrentActiveMontage _returnvalue)))

(event Custom|Server_GetDamage
  (if (< (Variables|STATS|GetHealth) 1.0)
    (Utilities|FlowControl|DoOnce false :!label _label
      (:Completed
        (Utilities|FlowControl|Delay 1.0)
        (bind _asgame_state_test (Utilities|Casting|CastToGameStateTest (Game|GetGameState)))
        (Default|ServerRoundWon _asgame_state_test (Variables|/Script/Engine.Pawn|GetPlayerState (Variables|REF|GetCharacter)))))
    (else
      (bind _output_get (Variables|STATS|SetHealth (- (Variables|STATS|GetHealth) 1.0)))
      (if (== _output_get 0.0)
        (goto _label)))))

(event Custom|Server_LaunchAnimTPS
  (params (SKMMontage :type Skeletal%20Mesh%20Component%20Object%20Reference) (MontageToPlay :type Anim%20Montage%20Object%20Reference))
  ;[0.15 0.15 0.15 0.5] Attack Anim System
  (CallFunction|MulticastLaunchAnimTPS SKMMontage MontageToPlay))

(event Custom|Server_Apply%20Damage
  (params (Blocker :type BP%20Third%20Person%20Character%20Main%20Object%20Reference) (Hit%20Location :type Vector) (Hit%20Bone%20Name :type Name) (Ratation :type Rotator))
  (bind _returnvalue (Transformation|GetActorForwardVector Blocker))
  (bind _returnvalue_2 (Transformation|GetActorLocation Blocker))
  (bind _postprocess (Variables|/Game/Core/Character/BP_ThirdPersonCharacterMain.BP_ThirdPersonCharacterMain_C|GetPostProcess Blocker))
  (bind _mesh (Variables|/Script/Engine.Character|GetMesh Blocker))
  (bind _character (Variables|REF|GetCharacter))
  (bind _status (Variables|/Game/Core/Character/BP_ThirdPersonCharacterMain.BP_ThirdPersonCharacterMain_C|GetStatus Blocker))
  (bind _returnvalue_3 (Transformation|GetActorLocation _character))
  (bind _returnvalue_4 (Math|Vector|GetUnitDirection(Vector) _returnvalue_2 _returnvalue_3))
  (bind _returnvalue_5 (Math|Vector|DotProduct _returnvalue_4 _returnvalue))
  (bind _returnvalue_6 (>= _returnvalue_5 0.5))
  ;[0.15 0.15 0.15 0.5] Apply Damage / check conditions (blocking,parry,behind ?)
  (Development|PrintString (Utilities|String|Append " Block Angle : " (Utilities|String|ToString(Boolean) _returnvalue_6) "Dot : " (Utilities|String|ToString(Float) _returnvalue_5) " State : " (Utilities|String|EnumtoString _status)) true true "(R=0.000000,G=0.660000,B=1.000000,A=1.000000)" 2e+01)
  (if _returnvalue_6
    (if (Utilities|Enum|Equal(Enum) _status "NewEnumerator6")
      (Development|PrintString "Stun")
      (CallFunction|MulticastSuccessParry _mesh)
      (CallFunction|ServerStun)
      (elif (Utilities|Enum|NotEqual(Enum) _status "NewEnumerator3")
        (Development|PrintString "Damage" :!label _label)
        (CallFunction|ServerGetDamage)
        (if (== (Variables|STATS|GetHealth) 2.0)
          (Rendering|Material|SetScalarParameterValue (Variables|/Game/Core/Character/BP_ThirdPersonCharacterMain.BP_ThirdPersonCharacterMain_C|GetPostProcess Blocker) "DamageStage" 1.0 :!class /Script/Engine.MaterialInstanceDynamic)
          (Rendering|AddorUpdateBlendable (Variables|/Game/Core/Character/BP_ThirdPersonCharacterMain.BP_ThirdPersonCharacterMain_C|GetFollowCamera Blocker) _postprocess 1.0 :!class /Script/Engine.CameraComponent :!label _label_2)
          (elif (== (Variables|STATS|GetHealth) 1.0)
            (Rendering|Material|SetScalarParameterValue _postprocess "DamageStage" 2.0 :!class /Script/Engine.MaterialInstanceDynamic)
            (goto _label_2)
            (else
              _)))
        (CallFunction|MulticastHItSound Hit%20Location Ratation Hit%20Bone%20Name Blocker)
        (else
          (CallFunction|MulticastSuccessParry _mesh))))
    (else
      (goto _label))))

(event EventBeginPlay
  ;[0.15 0.15 0.15 0.5] BeginPlay
  (bind _asbp_third_person_character_main (Utilities|Casting|CastToBP_ThirdPersonCharacterMain (Components|GetOwner)))
  (Variables|REF|SetCharacter _asbp_third_person_character_main))

(event Input|MouseEvents|RightMouseButton
  (params (Key :type Key%20Structure :default "None"))
  ;[0.15 0.15 0.15 0.5] Block/Input
  (:Pressed
    (CallFunction|ServerParryStates)))

(event Input|MouseEvents|LeftMouseButton
  (params (Key :type Key%20Structure :default "None"))
  (bind _character (Variables|REF|GetCharacter))
  ;[0.15 0.15 0.15 0.5] Attack / Input
  (:Pressed
    (if (Utilities|Enum|Equal(Enum) (Variables|/Game/Core/Character/BP_ThirdPersonCharacterMain.BP_ThirdPersonCharacterMain_C|GetStatus (Variables|REF|GetCharacter)) "NewEnumerator4")
      (Variables|/Game/Core/Character/BP_ThirdPersonCharacterMain.BP_ThirdPersonCharacterMain_C|SetStatus (Variables|REF|GetCharacter) "NewEnumerator2")
      ;;[0 1 1] @TODO : Refacto
      (CallFunction|GenerateRandomAnimation)
      (Utilities|FlowControl|Sequence
        (:then_0
          (CallFunction|ClientLaunchAnimFPS (.OutItem (Utilities|Array|Random (Variables|Animations|GetAnimsFPS))))
          (CallFunction|ServerLaunchAnimTPS (Variables|/Script/Engine.Character|GetMesh (Variables|REF|GetCharacter)) (.OutItem (Utilities|Array|Random (Variables|Animations|GetAnimTPS)))))
        (:then_1
          (Utilities|FlowControl|Delay (Variables|BlockSettings|GetDelayAttack))
          (if (Utilities|Enum|Equal(Enum) (Variables|/Game/Core/Character/BP_ThirdPersonCharacterMain.BP_ThirdPersonCharacterMain_C|GetStatus _character) "NewEnumerator2")
            (Variables|/Game/Core/Character/BP_ThirdPersonCharacterMain.BP_ThirdPersonCharacterMain_C|SetStatus _character "NewEnumerator4")))))))

(fn GenerateRandomAnimation
  (bind _returnvalue (CallFunction|GenerateIndex :!label _label))
  (if (== (Variables|Function|GetLastRandom) _returnvalue)
    (goto _label)
    (else
      (bind _output_get (Variables|Function|SetLastRandom _returnvalue))
      (return (Utilities|Array|Get(acopy) (Variables|Animations|GetAnimTPS) _output_get) (Utilities|Array|Get(acopy) (Variables|Animations|GetAnimsFPS) _output_get)))))

(fn GenerateIndex
  (return (Math|Random|RandomIntegerinRange 0 (Utilities|Array|LastIndex (Variables|Animations|GetAnimTPS)))))

(fn OnRepBlocking?)

(fn OnRepPB)

(fn OnRepHealth)

(fn OnRepHitActor)

(fn AnyDamage
  (params (Damage :type Integer) (Hit%20Bone%20Name :type Name) (Damage%20Causer :type Actor%20Object%20Reference) (Bloquer :type BP%20Third%20Person%20Character%20Main%20Object%20Reference))
  (Variables|Démenbrement|SetDamage%20Causer Bloquer)
  (Variables|Démenbrement|SetHit%20Bone%20Name Hit%20Bone%20Name)
  (Variables|Démenbrement|SetDamage Damage)
  (CallFunction|Dissmebrement Bloquer "None")
  (return))

(fn RenameBoneName
  (switch name (Variables|Démenbrement|GetHit%20Bone%20Name)
    (:Pelvis
      _)
    (:Spine_02
      _)
    (:Spine_03
      _)
    (:Neck_01
      _))
  (Variables|Démenbrement|SetHit%20Bone%20Name "None"))

(fn ApplyDamagetoBone
  (if (.ReturnValue (Utilities|Map|Find (Variables|Démenbrement|GetBreakableBones/Durability) (Variables|Démenbrement|GetHit%20Bone%20Name)))
    (Utilities|Map|Add (Variables|Démenbrement|GetBreakableBones/Durability) (Variables|Démenbrement|GetHit%20Bone%20Name) (- 0 (Variables|Démenbrement|GetDamage)))
    (return (< (.Value (Utilities|Map|Find (Variables|Démenbrement|GetBreakableBones/Durability) (Variables|Démenbrement|GetHit%20Bone%20Name))) 0))))

(fn Dissmebrement
  (params (Target :type Character%20Object%20Reference) (Hit%20Bones%20Name :type Name))
  (bind _asbp_third_person_character_main (Utilities|Casting|CastToBP_ThirdPersonCharacterMain Target))
  (bind _hit_bone_name (Variables|Démenbrement|GetHit%20Bone%20Name))
  (bind _mesh (Variables|/Script/Engine.Character|GetMesh Target))
  (bind _returnvalue (Transformation|GetSocketTransform _mesh Hit%20Bones%20Name "RTS_World"))
  (Components|SkinnedMesh|HideBonebyName _mesh Hit%20Bones%20Name "PBO_None")
  (Development|PrintString (Utilities|String|ToString(Name) Hit%20Bones%20Name) true true "(R=1.000000,G=0.000000,B=0.820275,A=1.000000)" 1e+01)
  (Niagara|SpawnSystemAttached "/Game/RealisticBlood/Dripping/Niagara/NS_Dripping_High.NS_Dripping_High" _mesh Hit%20Bones%20Name (.location _returnvalue) (.rotation _returnvalue) "KeepWorldPosition" true)
  (Niagara|SpawnSystemAttached "/Game/RealisticBlood/Dripping/Niagara/NS_Dripping_Splash_High.NS_Dripping_Splash_High" (Variables|/Script/Engine.Character|GetMesh Target) (Variables|Démenbrement|GetHit%20Bone%20Name) (.location _returnvalue) (.rotation _returnvalue) "KeepWorldPosition" true)
  (Niagara|SpawnSystemAttached "/Game/RealisticBlood/Splatter/Niagara/NS_Splatter_Directional_01_Decal.NS_Splatter_Directional_01_Decal" (Variables|/Script/Engine.Character|GetMesh Target) (Variables|Démenbrement|GetHit%20Bone%20Name) (.location _returnvalue) (.rotation _returnvalue) "KeepWorldPosition" true)
  (Niagara|SpawnSystemAttached "/Game/RealisticBlood/Hit/Niagara/NS_BulletHit_High.NS_BulletHit_High" (Variables|/Script/Engine.Character|GetMesh Target) _hit_bone_name (.location _returnvalue) (.rotation _returnvalue) "KeepWorldPosition" true)
  (Variables|Démenbrement|SetHasSpineBroken (== _hit_bone_name "spine_01"))
  (Utilities|Array|Add (Variables|Default|GetBrokenBones) (Variables|Démenbrement|GetHit%20Bone%20Name))
  (Physics|SetSimulatePhysics (Variables|/Script/Engine.Character|GetMesh Target) true)
  (Physics|SetSimulatePhysics (Variables|/Game/Core/Character/BP_ThirdPersonCharacterMain.BP_ThirdPersonCharacterMain_C|GetMesh_Local _asbp_third_person_character_main) true)
  (Transformation|DetachFromComponent (Variables|/Game/Core/Character/BP_ThirdPersonCharacterMain.BP_ThirdPersonCharacterMain_C|GetLocal_Katana _asbp_third_person_character_main) "KeepRelative" "KeepRelative" "KeepRelative" true)
  (Input|DisableInput _asbp_third_person_character_main (Game|GetPlayerController 0)))