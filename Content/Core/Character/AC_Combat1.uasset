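; Multiplayer katana combat component for the third-person character, handling attacks, blocking, parrying, stun and health.
; Clicks replicate non-repeating random montages to first-person and body meshes, or open a timed parry-then-block window with cooldown and blade colour cues.
; A camera-based box trace applies one hit per swing.
; Facing angle decides whether hits are parried (stunning the attacker), blocked or damaging, with depleted health awarding the opponent the round.
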(event Custom|Server_Parry
  (params (Target :type BP%20Third%20Person%20Character%20Main%20Object%20Reference))
  ;[0.15 0.15 0.15 0.5] Parry
  (CallFunction|MulticastParry Target))

(event Custom|Multicast_parry
  (params (Target :type BP%20Third%20Person%20Character%20Main%20Object%20Reference))
  ;[0.15 0.15 0.15 0.5] Parry
  (CallFunction|Stun (Variables|/Game/Core/Character/BP_ThirdPersonCharacterMain.BP_ThirdPersonCharacterMain_C|GetAC_Combat Target) (Variables|BlockSettings|GetParryStun)))

(event Custom|Multicast_Blocked
  (params (Target :type BP%20Third%20Person%20Character%20Main%20Object%20Reference))
  ;[0.15 0.15 0.15 0.5] Blocked
  (Utilities|FlowControl|Sequence
    (:then_0
      (Animation|Montage|PlayMontage (Variables|/Game/Core/Character/BP_ThirdPersonCharacterMain.BP_ThirdPersonCharacterMain_C|GetMesh_Local Target) "/Game/Art/Characters/Mannequins/Anims/FPSAnim/AM_Parry_Hit.AM_Parry_Hit"))
    (:then_1
      (Animation|Montage|PlayMontage (Variables|/Script/Engine.Character|GetMesh Target) "/Game/Core/Character/Animations/AM_BlockHit.AM_BlockHit"))))

(event Custom|Server_AttackTrace
  (bind _character (Variables|REF|GetCharacter))
  (bind _followcamera (Variables|/Game/Core/Character/BP_ThirdPersonCharacterMain.BP_ThirdPersonCharacterMain_C|GetFollowCamera _character))
  (bind _returnvalue (Math|Vector|GetForwardVector _followcamera))
  (bind _returnvalue_2 (Transformation|GetWorldLocation _followcamera))
  (bind _returnvalue_3 (* _returnvalue 4e+01))
  (bind _returnvalue_4 (+ _returnvalue_2 _returnvalue_3))
  ;[0.15 0.15 0.15 0.5] Attack Trace / Box trace when attack
  (bind _outhits (Class|KismetSystemLibrary|BoxTraceMulti _returnvalue_4 (- _returnvalue_4 "0.000000,0.000000,100.000000") "40.000000,50.000000,50.000000" (Math|Rotator|FindLookatRotation _returnvalue_4 (Transformation|GetWorldLocation _followcamera)) "TraceTypeQuery2" false 0 "ForOneFrame" true))
  (for _array_element _outhits
    (bind _asbp_third_person_character_main (Utilities|Casting|CastToBP_ThirdPersonCharacterMain (.HitActor (Collision|BreakHitResult _array_element))))
    (if (!= _asbp_third_person_character_main self)
      (if (Variables|CombatBools|GetHitActor)
        (Variables|CombatBools|SetHitActor false)
        (CallFunction|ServerApplyDamage (Variables|/Game/Core/Character/BP_ThirdPersonCharacterMain.BP_ThirdPersonCharacterMain_C|GetAC_Combat _asbp_third_person_character_main) (Transformation|GetActorLocation (Variables|REF|GetCharacter)) (Variables|REF|GetCharacter))))))

(event Custom|Stun
  (params (Duration :type Float%20%28single-precision%29))
  ;[0.15 0.15 0.15 0.5] Stun
  (if (> (Variables|/Game/Core/Character/BP_ThirdPersonCharacterMain.BP_ThirdPersonCharacterMain_C|GetStun? (Variables|REF|GetCharacter)) 0.0)
    (Variables|/Game/Core/Character/BP_ThirdPersonCharacterMain.BP_ThirdPersonCharacterMain_C|SetStun? (Variables|REF|GetCharacter) Duration)
    (else
      (Variables|/Game/Core/Character/BP_ThirdPersonCharacterMain.BP_ThirdPersonCharacterMain_C|SetStun? (Variables|REF|GetCharacter) Duration)
      (bind _returnvalue (Utilities|Time|SetTimerbyEvent (delegate Custom|CountStun) 0.01 true))
      (Variables|Default|SetStun%20Timer _returnvalue))))

(event Custom|CountStun
  (bind _character (Variables|REF|GetCharacter))
  ;[0.15 0.15 0.15 0.5] Stun
  (if (> (Variables|/Game/Core/Character/BP_ThirdPersonCharacterMain.BP_ThirdPersonCharacterMain_C|GetStun? (Variables|REF|GetCharacter)) 0.0)
    (Variables|/Game/Core/Character/BP_ThirdPersonCharacterMain.BP_ThirdPersonCharacterMain_C|SetStun? _character (- (Variables|/Game/Core/Character/BP_ThirdPersonCharacterMain.BP_ThirdPersonCharacterMain_C|GetStun? _character) 0.01))
    (if (<= (Variables|/Game/Core/Character/BP_ThirdPersonCharacterMain.BP_ThirdPersonCharacterMain_C|GetStun? (Variables|REF|GetCharacter)) 0.0)
      (if (Utilities|Time|IsValidTimerHandle (Variables|Default|GetStun%20Timer)) :!label _label
        (Utilities|Time|ClearandInvalidateTimerbyHandle (Variables|Default|GetStun%20Timer))))
    (else
      (Variables|/Game/Core/Character/BP_ThirdPersonCharacterMain.BP_ThirdPersonCharacterMain_C|SetStun? (Variables|REF|GetCharacter) 0.0)
      (goto _label))))

(event Custom|Server_Blocked
  (params (Target :type BP%20Third%20Person%20Character%20Main%20Object%20Reference))
  ;[0.15 0.15 0.15 0.5] Blocked
  (CallFunction|MulticastBlocked Target))

(event Custom|Server_Block
  (params (char :type BP%20Third%20Person%20Character%20Main%20Object%20Reference))
  ;[0.15 0.15 0.15 0.5] Block and Parry
  (CallFunction|MulticastBlock char)
  (Variables|/Game/Core/Character/BP_ThirdPersonCharacterMain.BP_ThirdPersonCharacterMain_C|SetBlocking? char true))

(event Custom|Multicast_Block
  (params (char :type BP%20Third%20Person%20Character%20Main%20Object%20Reference))
  (bind _mesh (Variables|/Script/Engine.Character|GetMesh char))
  (bind _returnvalue (Components|SkeletalMesh|GetAnimInstance _mesh))
  ;[0.15 0.15 0.15 0.5] Block and Parry
  (Animation|Montage|MontageStop _returnvalue 0.25 (Animation|Montage|GetCurrentActiveMontage _returnvalue)))

(event Custom|Server_ReleaseBlock
  (params (Char :type BP%20Third%20Person%20Character%20Main%20Object%20Reference))
  ;[0.15 0.15 0.15 0.5] Block and Parry
  (Variables|/Game/Core/Character/BP_ThirdPersonCharacterMain.BP_ThirdPersonCharacterMain_C|SetBlocking? Char false))

(event Custom|Server_GetDamage
  ;[0.15 0.15 0.15 0.5] Got hit / damaged finish round
  (if (< (Variables|STATS|GetHealth) 1.0)
    (bind _array_element (Utilities|Array|ForEachLoopwithBreak 0 :!label _label)
      (:LoopBody
        (if (!= (.AsBP%20Third%20Person%20Character%20Main (Utilities|Casting|CastToBP_ThirdPersonCharacterMain (Components|GetOwner))) _array_element)
          (Default|MulticastRoundWon (.AsBP%20Third%20Person%20Game%20Mode (Utilities|Casting|CastToBP_ThirdPersonGameMode (Game|GetGameMode))) (.AsBP%20Third%20Person%20Player%20Controller (Utilities|Casting|CastToBP_ThirdPersonPlayerController (Pawn|GetController _array_element))))
          (goto _label Break))))
    (else
      (bind _result (Math|Float|DecrementFloat (Variables|STATS|GetHealth))
        (:%20%20
          (bind _output_get (Variables|STATS|SetHealth _result))
          (Development|PrintString (Utilities|String|Append "Health: " (Utilities|String|ToString(Float) _output_get))))))))

(event Custom|ML_RequestAnim
  (params (MontageToPlay :type Anim%20Montage%20Object%20Reference) (Target :type BP%20Third%20Person%20Character%20Main%20Object%20Reference) (MontageToPlayFPS :type Anim%20Montage%20Object%20Reference))
  ;[0.15 0.15 0.15 0.5] Attack Anim/ replication
  (Utilities|FlowControl|Sequence
    (:then_0
      (Animation|Montage|PlayMontage (Variables|/Game/Core/Character/BP_ThirdPersonCharacterMain.BP_ThirdPersonCharacterMain_C|GetMesh_Local Target) MontageToPlayFPS))
    (:then_1
      (Animation|Montage|PlayMontage (Variables|/Script/Engine.Character|GetMesh Target) MontageToPlay
        (:OnNotifyBegin
          (Variables|Combatbools|SetCanAttack? true)
          (Default|ServerSwipeColor (Variables|REF|GetCharacter) (Variables|ColorSettings|GetKatana%20Normal%20Color)))))))

(event Custom|Server_SetPB
  (params (PB :type Boolean))
  ;[0.15 0.15 0.15 0.5] Block and Parry
  (Variables|CombatBools|SetPB PB))

(event Custom|RS_RequestAnim
  (params (MontageToPlay :type Anim%20Montage%20Object%20Reference) (Target :type BP%20Third%20Person%20Character%20Main%20Object%20Reference) (MontageToPlayFPS :type Anim%20Montage%20Object%20Reference))
  ;[0.15 0.15 0.15 0.5] Attack Anim/ replication
  (CallFunction|MLRequestAnim MontageToPlay Target MontageToPlayFPS)
  (Variables|CombatBools|SetHitActor true))

(event Custom|Server_Apply%20Damage
  (params (Attacker%20Location :type Vector) (Attacker :type BP%20Third%20Person%20Character%20Main%20Object%20Reference))
  (bind _character (Variables|REF|GetCharacter))
  ;[0.15 0.15 0.15 0.5] Apply Damage / check conditions (blocking,parry,behind ?)
  (if (< (Class|KismetMathLibrary|DegAcos (Math|Vector|DotProduct (Math|Rotator|GetRotationXVector (Math|Rotator|FindLookatRotation (Transformation|GetActorLocation _character) Attacker%20Location)) (Transformation|GetActorForwardVector _character))) (Variables|BlockSettings|GetBlock%20angle))
    (if (Variables|CombatBools|GetPB)
      ;;[0.15 0.15 0.15 0.5] Parry
      (Networking|SwitchHasAuthority
        (:Authority
          (CallFunction|ServerParry Attacker))
        (:Remote
          (CallFunction|MulticastParry)))
      (elif (Variables|/Game/Core/Character/BP_ThirdPersonCharacterMain.BP_ThirdPersonCharacterMain_C|GetBlocking? (Variables|REF|GetCharacter))
        ;;[0.15 0.15 0.15 0.5] Block
        (Networking|SwitchHasAuthority
          (:Authority
            (CallFunction|ServerBlocked (Variables|REF|GetCharacter)))
          (:Remote
            (CallFunction|MulticastBlocked (Variables|REF|GetCharacter))))
        (else
          (CallFunction|ServerGetDamage :!label _label))))
    (else
      (goto _label))))

(event EventBeginPlay
  ;[0.15 0.15 0.15 0.5] BeginPlay
  (bind _asbp_third_person_character_main (Utilities|Casting|CastToBP_ThirdPersonCharacterMain (Components|GetOwner)))
  (Variables|REF|SetCharacter _asbp_third_person_character_main))

(event Input|MouseEvents|RightMouseButton
  (params (Key :type Key%20Structure))
  ;[0.15 0.15 0.15 0.5] Block/Input
  (:Pressed
    (if (not (> (Variables|/Game/Core/Character/BP_ThirdPersonCharacterMain.BP_ThirdPersonCharacterMain_C|GetStun? (Variables|REF|GetCharacter)) 0.0))
      (if (not (Variables|CombatBools|GetBlockCD))
        (if (Variables|Combatbools|GetCanAttack?)
          (Variables|CombatBools|SetBlockCD true)
          (Default|ServerSwipeColor (Variables|REF|GetCharacter) (Variables|ColorSettings|GetKatana%20Parry%20Color))
          (CallFunction|ServerBlock (Variables|REF|GetCharacter))
          (CallFunction|ServerSetPB true)
          (Utilities|FlowControl|Delay (Variables|BlockSettings|GetParryDuration))
          (Default|ServerSwipeColor (Variables|REF|GetCharacter) (Variables|ColorSettings|GetKatana%20Block%20Color))
          (CallFunction|ServerSetPB false)
          (Utilities|FlowControl|Delay (Variables|BlockSettings|GetBlockDuration))
          (CallFunction|ServerReleaseBlock (Variables|REF|GetCharacter))
          (Default|ServerSwipeColor (Variables|REF|GetCharacter) (Variables|ColorSettings|GetKatana%20Normal%20Color))
          (Utilities|FlowControl|Delay (Variables|BlockSettings|GetBlockCooldown))
          (Variables|CombatBools|SetBlockCD false))))))

(event Input|MouseEvents|LeftMouseButton
  (params (Key :type Key%20Structure))
  ;[0.15 0.15 0.15 0.5] Attack / Input
  (:Pressed
    (if (not (> (Variables|/Game/Core/Character/BP_ThirdPersonCharacterMain.BP_ThirdPersonCharacterMain_C|GetStun? (Variables|REF|GetCharacter)) 0.0))
      (if (not (Variables|/Game/Core/Character/BP_ThirdPersonCharacterMain.BP_ThirdPersonCharacterMain_C|GetBlocking? (Variables|REF|GetCharacter)))
        (if (Variables|Combatbools|GetCanAttack?)
          (bind (_resultanim _resultanimfps) (CallFunction|GenerateRandomAnimation))
          (Default|ServerSwipeColor (Variables|REF|GetCharacter) (Variables|ColorSettings|GetKatana%20Attack%20Color))
          (Variables|Combatbools|SetCanAttack? false)
          (Networking|SwitchHasAuthority
            (:Authority
              (CallFunction|MLRequestAnim _resultanim (Variables|REF|GetCharacter) _resultanimfps)
              (Variables|CombatBools|SetHitActor true))
            (:Remote
              (CallFunction|RSRequestAnim _resultanim (Variables|REF|GetCharacter) _resultanimfps))))))))

(fn GenerateRandomAnimation
  (bind _returnvalue (CallFunction|GenerateIndex :!label _label))
  (if (== (Variables|Function|GetLastRandom) _returnvalue)
    (goto _label)
    (else
      (bind _output_get (Variables|Function|SetLastRandom _returnvalue))
      (return (Utilities|Array|Get(acopy) (Variables|Animations|GetCombatAnims) _output_get) (Utilities|Array|Get(acopy) (Variables|Animations|GetAnimsFPS) _output_get)))))

(fn GenerateIndex
  (return (Math|Random|RandomIntegerinRange 0 (Utilities|Array|LastIndex (Variables|Animations|GetCombatAnims)))))

(fn OnRepBlocking?)

(fn OnRepPB)

(fn OnRepHealth)

(fn OnRepHitActor)