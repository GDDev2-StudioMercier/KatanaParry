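; Dash ability that quickly moves the player a set distance, with a sound, cooldown timer and server-to-multicast replication.
; Grounded dashes follow movement input, while airborne or input-less dashes follow the camera's forward vector.
; A line trace shortens the dash at obstacles and scales its duration to match.
; Tick lerps the player there with sweep while fading the DashStrenght parameter on a dynamic post-process material.
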(event Custom|ResetDash
  (Variables|Default|SetElapsed 0.0)
  (Variables|Default|SetbIsDashing? false))

(event Custom|Server_Dash
  (CallFunction|MulticastDash))

(event Custom|Multicast_Dash
  (bind _cameraref (Variables|Default|GetCameraREF))
  (bind _player_ref (Variables|Default|GetPlayer%20REF))
  (bind _returnvalue (Transformation|GetActorLocation _player_ref))
  (bind _returnvalue_2 (Transformation|GetWorldLocation _cameraref))
  (if (and (not (Variables|Default|GetbIsDashing?)) (Variables|Default|GetbCanDash?))
    (Variables|Default|SetbIsDashing? true)
    (Variables|Default|SetbCanDash? false)
    (Audio|PlaySound2D "/Game/SFX/Player/dash_cue.dash_cue" 1.0 1.0 0.0 0 0)
    (Utilities|FlowControl|Sequence
      (:then_0
        (if (not (AI|Components|NavMovement|IsFalling (Variables|/Script/Engine.Character|GetCharacterMovement (Variables|Default|GetPlayer%20REF))))
          (Variables|Default|SetInitalLocation _returnvalue)
          (bind _asbp_third_person_character_main (Utilities|Casting|CastToBP_ThirdPersonCharacterMain _player_ref))
          (Variables|Default|SetAs%20BP%20Character%20Dash%20Test _asbp_third_person_character_main)
          (if (or (not (== (Variables|/Game/Core/Character/BP_ThirdPersonCharacterMain.BP_ThirdPersonCharacterMain_C|GetAction%20Value%20Y _asbp_third_person_character_main) 0.0)) (not (== (Variables|/Game/Core/Character/BP_ThirdPersonCharacterMain.BP_ThirdPersonCharacterMain_C|GetAction%20Value%20X _asbp_third_person_character_main) 0.0)))
            (Variables|Default|SetDesiredLocation (+ _returnvalue (* (+ (* (Transformation|GetActorForwardVector _player_ref) (.y (Math|Vector|Normalize (Math|Vector|MakeVector (Variables|/Game/Core/Character/BP_ThirdPersonCharacterMain.BP_ThirdPersonCharacterMain_C|GetAction%20Value%20X _asbp_third_person_character_main) (Variables|/Game/Core/Character/BP_ThirdPersonCharacterMain.BP_ThirdPersonCharacterMain_C|GetAction%20Value%20Y _asbp_third_person_character_main) 0.0)))) (* (Transformation|GetActorRightVector _player_ref) (.x (Math|Vector|Normalize (Math|Vector|MakeVector (Variables|/Game/Core/Character/BP_ThirdPersonCharacterMain.BP_ThirdPersonCharacterMain_C|GetAction%20Value%20X _asbp_third_person_character_main) (Variables|/Game/Core/Character/BP_ThirdPersonCharacterMain.BP_ThirdPersonCharacterMain_C|GetAction%20Value%20Y _asbp_third_person_character_main) 0.0))))) (Variables|Default|GetDashLenght))))
            (else
              (Variables|Default|SetInitalLocation _returnvalue_2 :!label _label)
              (Variables|Default|SetDesiredLocation (+ _returnvalue_2 (* (Math|Vector|GetForwardVector _cameraref) (Variables|Default|GetDashLenght))))))
          (else
            (goto _label)))
        (bind (_outhit _returnvalue_3) (Collision|LineTraceByChannel (Variables|Default|GetInitalLocation) (Variables|Default|GetDesiredLocation) "TraceTypeQuery1" false 0 "ForDuration"))
        (if _returnvalue_3
          (bind _output_get (Variables|Default|SetDesiredLocation (.ImpactPoint (Collision|BreakHitResult _outhit))))
          (Variables|Default|SetCalculedDuration (* (Variables|Default|GetBaseDuration) (/ (Math|Vector|Distance(Vector) (Variables|Default|GetInitalLocation) _output_get) (Variables|Default|GetDashLenght))))
          (else
            (Variables|Default|SetCalculedDuration (Variables|Default|GetBaseDuration)))))
      (:then_1
        (Utilities|FlowControl|DoOnce true) ; enters at Reset
      )
      (:then_2
        (Utilities|Time|SetTimerbyEvent (delegate Custom|ResetDashCooldown) (Variables|Default|GetDashCooldown))))))

(event Custom|ResetDashCooldown
  (Variables|Default|SetbCanDash? true))

(event Custom|InitDash
  (bind _returnvalue (Rendering|Material|CreateDynamicMaterialInstance "/Game/Effects/Dash/MM_Dash.MM_Dash" "None" "None" :!class /Script/Engine.KismetMaterialLibrary))
  (Variables|Default|SetPostProcessMID _returnvalue))

(event Input|EnhancedActionEvents|EnhancedInputActionIA_Dash
  (params (ActionValue :type Boolean) (ElapsedSeconds :type Float%20%28double-precision%29) (TriggeredSeconds :type Float%20%28double-precision%29) (InputAction :type Input%20Action%20Object%20Reference :default "/Game/Core/Character/Input/Actions/IA_Dash.IA_Dash"))
  (:Started
    (if (Utilities|Enum|NotEqual(Enum) (Variables|/Game/Core/Character/BP_ThirdPersonCharacterMain.BP_ThirdPersonCharacterMain_C|GetStatus (Variables|Default|GetAs%20BP%20Character%20Dash%20Test)) "NewEnumerator5")
      (Networking|SwitchHasAuthority
        (:Authority
          (CallFunction|MulticastDash))
        (:Remote
          (CallFunction|ServerDash))))))

(event EventTick
  (params (DeltaSeconds :type Float%20%28single-precision%29))
  (if (and (Variables|Default|GetbIsDashing?) (> (Variables|Default|GetCalculedDuration) (Variables|Default|GetElapsed)))
    (Variables|Default|SetElapsed (+ (Variables|Default|GetElapsed) (Utilities|Time|GetWorldDeltaSeconds)))
    (Transformation|SetActorLocation (Variables|Default|GetPlayer%20REF) (Math|Vector|Lerp(Vector) (Variables|Default|GetInitalLocation) (Variables|Default|GetDesiredLocation) (/ (Variables|Default|GetElapsed) (Variables|Default|GetCalculedDuration))) true false)
    (Rendering|Material|SetScalarParameterValue (Variables|Default|GetPostProcessMID) "DashStrenght" (Math|Float|Lerp 1.0 0.0 (/ (Variables|Default|GetElapsed) (Variables|Default|GetCalculedDuration))) :!class /Script/Engine.MaterialInstanceDynamic)
    (else
      (Utilities|FlowControl|DoOnce true
        (:Completed
          (CallFunction|ResetDash))))))

(fn Initialize
  (params (PlayerREF :type Character%20Object%20Reference) (CameraREF :type Camera%20Component%20Object%20Reference) (Action%20Value%20X :type Float%20%28double-precision%29) (Action%20Value%20Y :type Float%20%28double-precision%29))
  (Variables|Default|SetPlayer%20REF PlayerREF)
  (Variables|Default|SetCameraREF CameraREF)
  (Variables|Default|SetAction%20Value%20X Action%20Value%20X)
  (Variables|Default|SetAction%20Value%20Y Action%20Value%20Y))