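; Player-driven cyberpunk car that can also move vertically, with gravity switched off above a set world height.
; Tick turns throttle, steer and up input into Plane's physics velocity and interpolated banking and yaw, with Handbrake false while Space is held.
; It also animates wheels, steering and toggled windows, updates lights, and feeds speed and window positions to audio.
; The construction script applies body color, dirt, wheel glow and headlight color.
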(event EventTick
  (params (DeltaSeconds :type Float%20%28single-precision%29))
  (bind _returnvalue (Transformation|GetActorRotation))
  (bind _returnvalue_2 (Transformation|GetVelocity))
  (bind _returnvalue_3 (Input|AxisValues|GetUp))
  (bind _returnvalue_4 (Input|AxisValues|GetSteer))
  (bind _returnvalue_5 (Input|AxisValues|GetThrottle))
  (bind _returnvalue_6 (Input|AxisValues|GetSteer))
  (bind _returnvalue_7 (Input|AxisValues|GetThrottle))
  (bind _plane (Variables|Default|Getplane))
  (bind _handbrake (Variables|Animation|GetHandbrake))
  (bind _handbrake_2 (Variables|Animation|GetHandbrake))
  (bind _frontlights (Variables|Lights|GetFrontlights))
  (bind _frontlight_intensity (Variables|Lights|GetFrontLight%20Intensity))
  (bind _sc_enginesound (Variables|Default|GetSC_EngineSound))
  (bind _sc_windows (Variables|Default|GetSC_Windows))
  (bind _handbrake_3 (Variables|Animation|GetHandbrake))
  (bind _returnvalue_8 (Math|Conversions|ToFloat(Boolean) _handbrake_3))
  (bind _returnvalue_9 (Math|Vector|VectorLength _returnvalue_2))
  (bind _returnvalue_10 (Math|Conversions|ToFloat(Boolean) _frontlights))
  (bind _returnvalue_11 (Math|Conversions|ToFloat(Boolean) _handbrake))
  (bind _returnvalue_12 (Math|Conversions|ToFloat(Boolean) _handbrake_2))
  (bind _returnvalue_13 (* _returnvalue_5 15.0))
  (bind _returnvalue_14 (* _returnvalue_4 1e+01))
  (bind _returnvalue_15 (* _returnvalue_4 3e+01))
  (bind _returnvalue_16 (Math|Float|Absolute(Float) _returnvalue_9))
  (bind _returnvalue_17 (+ _returnvalue_14 _returnvalue_13))
  (bind _returnvalue_18 (* _returnvalue_12 _returnvalue_7))
  (bind _returnvalue_19 (* _returnvalue_11 _returnvalue_17))
  (bind _returnvalue_20 (Math|Rotator|MakeRotator _returnvalue_19 _returnvalue_15 0.0))
  (bind _output_get (Variables|Animation|SetSpeed (Math|Interpolation|FInterpTo (Variables|Animation|GetSpeed) (* (* (Input|AxisValues|GetThrottle) _returnvalue_8) (Variables|Animation|GetForward%20Speed) 0.05) DeltaSeconds 1.0)))
  (Physics|SetEnableGravity _plane (not (> (.z (Transformation|GetWorldLocation _plane)) 4e+02)))
  (Variables|Default|SetDelta%20seconds DeltaSeconds)
  (Physics|SetPhysicsLinearVelocity (Variables|Default|Getplane) (+ (Transformation|GetVelocity) (* (* (Math|Vector|RotateVector (Math|Vector|MakeVector (* (* (Input|AxisValues|GetSteer) _returnvalue_8) (Variables|Animation|GetSteer%20Push) -0.05) (Math|Float|SelectFloat _output_get 0.0 _handbrake_3) (Math|Float|SelectFloat (* _returnvalue_8 _returnvalue_3) (* _returnvalue_8 (* _returnvalue_3 5.0)) (== _returnvalue_3 -1.0))) (Math|Rotator|MakeRotator 0.0 0.0 (.yaw (Transformation|GetActorRotation)))) (Variables|Animation|GetMovement%20speed)) (Variables|Default|GetDelta%20seconds))) false "None")
  (Transformation|SetActorRotation (Math|Rotator|MakeRotator (.roll (Math|Interpolation|RInterpTo (Math|Rotator|MakeRotator (.roll _returnvalue) (.pitch _returnvalue) (.yaw _returnvalue)) (Math|Rotator|MakeRotator (.roll _returnvalue_20) (.pitch _returnvalue_20) (+ (.yaw _returnvalue) (* (* (Math|Float|SelectFloat -1.0 1.0 (== _returnvalue_5 -1.0)) (Input|AxisValues|GetSteer)) (Variables|Animation|GetRotation%20Speed)))) (Variables|Default|GetDelta%20seconds) 1.0)) (.pitch (Math|Interpolation|RInterpTo (Math|Rotator|MakeRotator (.roll _returnvalue) (.pitch _returnvalue) (.yaw _returnvalue)) (Math|Rotator|MakeRotator (.roll _returnvalue_20) (.pitch _returnvalue_20) (+ (.yaw _returnvalue) (* (* (Math|Float|SelectFloat -1.0 1.0 (== _returnvalue_5 -1.0)) (Input|AxisValues|GetSteer)) (Variables|Animation|GetRotation%20Speed)))) (Variables|Default|GetDelta%20seconds) 1.0)) (.yaw (Math|Interpolation|RInterpTo (Math|Rotator|MakeRotator (.roll _returnvalue) (.pitch _returnvalue) (.yaw _returnvalue)) (Math|Rotator|MakeRotator (.roll _returnvalue_20) (.pitch _returnvalue_20) (+ (.yaw _returnvalue) (* (* (Math|Float|SelectFloat -1.0 1.0 (== _returnvalue_5 -1.0)) (Input|AxisValues|GetSteer)) (Variables|Animation|GetRotation%20Speed)))) (Variables|Default|GetDelta%20seconds) 1.0))))
  (bind _output_get_2 (Variables|Animation|SetWheelRL (Math|Interpolation|FInterpTo (Variables|Animation|GetWheelRL) (* _returnvalue_18 1e+01) (Utilities|Time|GetWorldDeltaSeconds) 2.5)))
  (Transformation|SetRelativeRotation (Variables|Default|GetRR) (Math|Rotator|MakeRotator _output_get_2 0.0 0.0) false false)
  (bind _output_get_3 (Variables|Animation|SetWheelRR (Math|Interpolation|FInterpTo (Variables|Animation|GetWheelRR) (* _returnvalue_18 1e+01) (Utilities|Time|GetWorldDeltaSeconds) 2.5)))
  (Transformation|SetRelativeRotation (Variables|Default|GetRL) (Math|Rotator|MakeRotator _output_get_3 0.0 0.0) false false)
  (bind _output_get_4 (Variables|Animation|SetSteeringWheelRot (Math|Interpolation|FInterpTo (Variables|Animation|GetSteeringWheelRot) (* _returnvalue_6 55.0) (Utilities|Time|GetWorldDeltaSeconds) 4.0)))
  (Transformation|SetRelativeRotation (Variables|Default|GetSteeringWheel) (Math|Rotator|MakeRotator 0.0 _output_get_4 0.0) false false)
  (bind _output_get_5 (Variables|Animation|SetWheelFL (Math|Interpolation|FInterpTo (Variables|Animation|GetWheelFL) (* _returnvalue_6 15.0) (Utilities|Time|GetWorldDeltaSeconds) 2.5)))
  (Transformation|SetRelativeRotation (Variables|Default|GetFL) (Math|Rotator|MakeRotator 0.0 _output_get_5 0.0) false false)
  (bind _output_get_6 (Variables|Animation|SetWheelFR (Math|Interpolation|FInterpTo (Variables|Animation|GetWheelFR) (* _returnvalue_6 15.0) (Utilities|Time|GetWorldDeltaSeconds) 2.5)))
  (Transformation|SetRelativeRotation (Variables|Default|GetFR) (Math|Rotator|MakeRotator 0.0 _output_get_6 0.0) false false)
  (bind _output_get_7 (Variables|Animation|SetLeft%20Glass (Math|Interpolation|FInterpTo (Variables|Animation|GetLeft%20Glass) (Math|Conversions|ToFloat(Boolean) (Variables|Animation|GetLeftGlass)) (Utilities|Time|GetWorldDeltaSeconds) 2.8)))
  (Transformation|SetRelativeLocationAndRotation (Variables|Default|GetGlassL) (Math|Vector|MakeVector (+ (* _output_get_7 (- 97.534981 88.559753)) 88.559753) (+ (* _output_get_7 (- 10.753048 10.770735)) 10.770735) (+ (* _output_get_7 (- 70.079819 98.512093)) 98.512093)) (Math|Rotator|MakeRotator (+ (* _output_get_7 (- 0.574241 -0.176987)) -0.176987) (+ (* _output_get_7 (- 18.555138 19.656996)) 19.656996) (+ (* _output_get_7 (- 1.295261 -0.43816)) -0.43816)) false false)
  (Audio|Parameter|SetFloatParameter _sc_windows "Glass L" (+ (* _output_get_7 (- 70.079819 98.512093)) 98.512093) :!class /Script/Engine.AudioComponent)
  (bind _output_get_8 (Variables|Animation|SetRight%20Glass (Math|Interpolation|FInterpTo (Variables|Animation|GetRight%20Glass) (Math|Conversions|ToFloat(Boolean) (Variables|Animation|GetRightGlass)) (Utilities|Time|GetWorldDeltaSeconds) 2.8)))
  (Transformation|SetRelativeLocationAndRotation (Variables|Default|GetGlassR) (Math|Vector|MakeVector (+ (* _output_get_8 (- -97.534981 -88.559753)) -88.559753) (+ (* _output_get_8 (- 10.753048 10.770735)) 10.770735) (+ (* _output_get_8 (- 70.079819 98.512093)) 98.512093)) (Math|Rotator|MakeRotator (+ (* _output_get_8 (- 0.574241 -0.176987)) -0.176987) (+ (* _output_get_8 (- -18.555138 -19.656996)) -19.656996) (+ (* _output_get_8 (- 1.295261 -0.43816)) -0.43816)) false false)
  (Audio|Parameter|SetFloatParameter _sc_windows "Glass R" (+ (* _output_get_8 (- 70.079819 98.512093)) 98.512093) :!class /Script/Engine.AudioComponent)
  (if (or (Math|Boolean|Equal(Boolean) (Variables|Animation|GetHandbrake) false) (== (Input|AxisValues|GetThrottle) -1.0))
    (Variables|Lights|Setstoplights 3e+02)
    (else
      (Variables|Lights|Setstoplights 0.0)))
  (Rendering|Components|Light|SetIntensity (Variables|Default|GetPointLight12) (Variables|Lights|Getstoplights))
  (Rendering|Components|Light|SetIntensity (Variables|Default|GetFrontLight4) (* _returnvalue_10 _frontlight_intensity))
  (Rendering|Components|Light|SetIntensity (Variables|Default|GetSpotLight) (* _returnvalue_10 (* _frontlight_intensity 8e+02)))
  (Audio|Parameter|SetFloatParameter _sc_enginesound "RPM" _returnvalue_16 :!class /Script/Engine.AudioComponent)
  (Audio|Components|Audio|SetPitchMultiplier _sc_enginesound (* (+ (/ _returnvalue_16 9e+03) 0.2) 3.0)))

(event Input|AxisEvents|InputAxisLookUp
  (params (AxisValue :type Float%20%28single-precision%29))
  (Transformation|AddRelativeRotation (Variables|Default|GetSpringArm) (Math|Rotator|MakeRotator 0.0 AxisValue (stale Input|AxisEvents|InputAxisLookRight AxisValue)) false false))

(event Input|AxisEvents|InputAxisLookRight
  (params (AxisValue :type Float%20%28single-precision%29))
  (Transformation|AddRelativeRotation (Variables|Default|GetSpringArm) (Math|Rotator|MakeRotator 0.0 (stale Input|AxisEvents|InputAxisLookUp AxisValue) AxisValue) false false))

(event Input|KeyboardEvents|SpaceBar
  (params (Key :type Key%20Structure :default "None"))
  (:Pressed
    (Variables|Animation|SetHandbrake false))
  (:Released
    (Variables|Animation|SetHandbrake true)))

(event Input|KeyboardEvents|F
  (params (Key :type Key%20Structure :default "None"))
  (:Pressed
    (bind _isa (Utilities|FlowControl|FlipFlop)
      (:A
        _)
      (:B
        _))
    (Variables|Animation|SetLeftGlass _isa)))

(event Input|KeyboardEvents|R
  (params (Key :type Key%20Structure :default "None"))
  (:Pressed
    (bind _isa (Utilities|FlowControl|FlipFlop)
      (:A
        _)
      (:B
        _))
    (Variables|Animation|SetRightGlass _isa)))

(event Input|KeyboardEvents|T
  (params (Key :type Key%20Structure :default "None"))
  (:Pressed
    (bind _isa (Utilities|FlowControl|FlipFlop)
      (:A
        _)
      (:B
        _))
    (Variables|Lights|SetFrontlights _isa)))

(fn ConstructionScript
  (bind _fl (Variables|Default|GetFL))
  (bind _wheel_emissive (Variables|Material|GetWheel%20Emissive))
  (Rendering|Material|SetVectorParameterValueonMaterials (Variables|Default|GetBody) "param" (Math|Conversions|ToVector(LinearColor) (Variables|Material|GetBody%20Color)))
  (Rendering|Material|SetScalarParameterValueonMaterials _fl "Dirt Level" (Variables|Material|GetDirt%20Level))
  (Rendering|Material|SetVectorParameterValueonMaterials _fl "Emissive Color" (Math|Conversions|ToVector(LinearColor) _wheel_emissive))
  (Rendering|Components|Light|SetLightColor (Variables|Default|GetPointLight10) _wheel_emissive true)
  (Rendering|Components|Light|SetLightColor (Variables|Default|GetSpotLight) (Variables|Default|GetFrontlight) true))