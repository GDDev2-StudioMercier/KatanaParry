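; Round system component that tracks each player's round wins in a 1v1 match, first to three.
; RoundWon increments the winner's counter by net player index, then either triggers the multicast match win, which shows the victory menu, or reloads the SetDress_1v1 level for the next round.
; A separate authority-only event forwards the winner to the game mode's MulticastRoundWon.
; The counters' OnRep functions are empty.
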(event Custom|RoundReset
  (Utilities|Casting|CastToGI_AdvancedKatanaParry (Game|GetGameInstance))
  (Game|OpenLevel(byObjectReference) "/Game/Maps/SetDress/SetDress_1v1.SetDress_1v1"))

(event Custom|RoundWon
  (params (Winner :type BP%20Third%20Person%20Player%20Controller%20Object%20Reference))
  (switch int (Class|AdvancedSessionsLibrary|GetNetPlayerIndex Winner)
    (:0
      (bind _result (Math|Integer|IncrementInt (Variables|Default|GetPlayer1RoundsWon))
        (:%20%20
          (if (>= _result 3)
            (CallFunction|MulticastMatchWon :!label _label)
            (else
              (CallFunction|RoundReset :!label _label_2))))))
    (:1
      (bind _result_2 (Math|Integer|IncrementInt (Variables|Default|GetPlayer2RoundsWon))
        (:%20%20
          (if (>= _result_2 3)
            (goto _label)
            (else
              (goto _label_2))))))))

(event Custom|Multicast_MatchWon
  (bind _returnvalue (UserInterface|CreateWidget (Variables|Default|GetVictoryMenuClass)))
  (bind _output_get (Variables|Default|SetVictoryMenuObject _returnvalue))
  (UserInterface|Viewport|AddtoViewport _output_get 0))

(event Custom|CustomEvent
  (Networking|SwitchHasAuthority
    (:Authority
      (Default|MulticastRoundWon (.AsBP%20Third%20Person%20Game%20Mode (Utilities|Casting|CastToBP_ThirdPersonGameMode (Game|GetGameMode))) (Variables|Default|GetWinner)))))

(fn OnRepPlayer1RoundsWon)

(fn OnRepPlayer2RoundsWon)